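; BP_Famine_Dummy is a melee enemy unit Blueprint that drives montages for Famine's two skeletal meshes, Main and Head.
; On BeginPlay it listens for the Unit.Ability.BasicAttack gameplay event and plays the attack montage on Main and the matching one on Head.
; A Playdeadmontage event starts the death montages on both meshes in the same way.
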(event `self.ReceiveBeginPlay`
  (`parent.ReceiveBeginPlay`)
  (`AbilityAsync_WaitGameplayEvent.WaitGameplayEventToActor` null (struct :`TagName` "Unit.Ability.BasicAttack")
    (:`EventReceived`
      (`|PlayMontage` (`self.Main`) "/Game/_Externel_Asset/BlackStormAssets/Monster/Famine/Ani/AM_Famine.AM_Famine" 1.0 0.0 "None" false
        (:`then`
          (`|PlayMontage` (`self.Head`) "/Game/_Externel_Asset/BlackStormAssets/Monster/Famine/Ani/AM_Famine_Head.AM_Famine_Head" 1.0 0.0 "None" false))))))

(event `Playdeadmontage`
  (`|PlayMontage` (`self.Main`) "/Game/_Externel_Asset/BlackStormAssets/Monster/Famine/Ani/AM_Famine_Main_DIe.AM_Famine_Main_DIe" 1.0 0.0 "None" false
    (:`then`
      (`|PlayMontage` (`self.Head`) "/Game/_Externel_Asset/BlackStormAssets/Monster/Famine/Ani/AM_Famine_Head_Die.AM_Famine_Head_Die" 1.0 0.0 "None" false))))

(fn `UserConstructionScript`
  (`parent.UserConstructionScript`))