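; Pooled skill actor for a persistent area-of-effect skill, handling its lasting visual and sound effects.
; On activation from the pool, it runs the parent logic, then async-loads the persistent VFX and SFX referenced in its Config.
; Each loaded asset is assigned to the actor's Niagara or audio component and activated.
; This graph has no area-effect logic of its own; overlap and tick events are unused.
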(event `self.OnActivatedFromPool`
  (bind (_actorclass _actortype _effects _spawnlocationpolicy _targetpolicy _speed _maxrange _lifespan _hitsperlifespan _radius _indicatordecalmaterial _montage _visualasset) (break `HeroSpawnableConfig` (`self.Config`)))
  (bind _persistentvfx (`DataAsset_SkillVisualData.PersistentVFX` _visualasset))
  (bind _persistentsfx (`DataAsset_SkillVisualData.PersistentSFX` _visualasset))
  (`parent.OnActivatedFromPool`)
  (`|ExecutionSequence`
    (:`then_0`
      (bind _object (`|LoadAsset` _persistentvfx)
        (:`Completed`
          (`/Engine/EditorBlueprintResources/StandardMacros.IsValid` _object
            (:`Is Valid`
              (`NiagaraComponent.SetAsset` (`self.ActorVFXComponent`) (`|ConvertAsset` _persistentvfx) true)
              (`ActorComponent.Activate` (`self.ActorVFXComponent`) true))))))
    (:`then_1`
      (`|LoadAsset` _persistentsfx
        (:`Completed`
          (`AudioComponent.SetSound` (`self.ActorSFXComponent`) (`|ConvertAsset` _persistentsfx))
          (`ActorComponent.Activate` (`self.ActorSFXComponent`) true))))))

(fn `UserConstructionScript`)