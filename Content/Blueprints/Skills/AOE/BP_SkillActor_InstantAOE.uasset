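; Skill actor for an instant area-of-effect skill, handling its collision sizing and impact feedback.
; On BeginPlay it calls the parent, then scales the collision component by the runtime scale multiplier.
; It async-loads the impact VFX and SFX from Config, spawning a pooled, equally scaled Niagara system at its location and a 2D sound.
; OnInstantHit is empty, and no hit logic lives in this graph.
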(event `self.ReceiveBeginPlay`
  (bind _returnvalue (`self.GetRuntimeScaleMultiplier`))
  (bind _collisioncomponent (`self.CollisionComponent`))
  (bind (_actorclass _actortype _effects _spawnlocationpolicy _targetpolicy _speed _maxrange _lifespan _hitsperlifespan _radius _indicatordecalmaterial _montage _visualasset) (break `HeroSpawnableConfig` (`self.Config`)))
  (bind _impactvfx (`DataAsset_SkillVisualData.ImpactVFX` _visualasset))
  (bind _impactsfx (`DataAsset_SkillVisualData.ImpactSFX` _visualasset))
  (`parent.ReceiveBeginPlay`)
  (`SceneComponent.SetWorldScale3D` _collisioncomponent (* (`self.GetRuntimeScaleMultiplier`) (`SceneComponent.K2_GetComponentScale` _collisioncomponent)))
  (`|ExecutionSequence`
    (:`then_0`
      (bind _object (`|LoadAsset` _impactvfx)
        (:`Completed`
          (`/Engine/EditorBlueprintResources/StandardMacros.IsValid` _object
            (:`Is Valid`
              (`NiagaraFunctionLibrary.SpawnSystemAtLocation` (`|ConvertAsset` _impactvfx) (`self.K2_GetActorLocation`) (struct) (`KismetMathLibrary.MakeVector` _returnvalue _returnvalue _returnvalue) true true "AutoRelease"))))))
    (:`then_1`
      (bind _object_2 (`|LoadAsset` _impactsfx)
        (:`Completed`
          (`/Engine/EditorBlueprintResources/StandardMacros.IsValid` _object_2
            (:`Is Valid`
              (`GameplayStatics.SpawnSound2D` (`|ConvertAsset` _impactsfx) 1.0 1.0 0.0 null))))))))

(event `self.OnInstantHit`
  (params (TargetActor :type "Actor Object Reference")))

(fn `UserConstructionScript`)