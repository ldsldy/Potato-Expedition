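; Test hero for exercising Gameplay Ability System abilities and movement through debug keys.
; WASD keys set flags that Tick turns into world-axis movement input.
; Key 1 activates the basic attack by tag, while key 2 has two handlers for sub and main skills, printing the results.
; Key 3 starts a looping timer, never cleared, that lerps camera FOV from 90 to 60.
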(event Custom|SetFOV
  (bind _output_get (Variables|Default|SetCurrentTime (+ (Variables|Default|GetCurrentTime) 0.1)))
  (Camera|SetFieldOfView (Variables|Default|GetCameraComponent) (Math|Float|Lerp 9e+01 6e+01 (Math|Float|Clamp(Float) _output_get))))

(event Collision|EventActorBeginOverlap
  (params (OtherActor :type Actor%20Object%20Reference)))

(event EventTick
  (params (DeltaSeconds :type Float%20%28single-precision%29))
  (Utilities|FlowControl|Sequence
    (:then_0
      (if (Variables|Default|GetbIsWTrigger)
        (Pawn|Input|AddMovementInput "-0.000000,-1.000000,0.000000" 1e+02 false)))
    (:then_1
      (if (Variables|Default|GetbIsSTrigger)
        (Pawn|Input|AddMovementInput "-0.000000,1.000000,0.000000" 1e+02 false)))
    (:then_2
      (if (Variables|Default|GetbIsATrigger)
        (Pawn|Input|AddMovementInput "-1.000000,0.000000,0.000000" 1e+02 false)))
    (:then_3
      (if (Variables|Default|GetbIsDTrigger)
        (Pawn|Input|AddMovementInput "1.000000,0.000000,0.000000" 1e+02 false)))))

(event Input|KeyboardEvents|DebugKey1
  (params (Key :type Key%20Structure :default "None") (ActionValue :type Input%20Action%20Value%20Structure))
  (:Pressed
    (bind _returnvalue (Class|PGAbilitySystemComponent|TryActivateAbilitybyTag (Variables|Default|GetPGAbilitySystemComponent) "(TagName=\"Input.BasicAttack\")"))
    (if _returnvalue
      (Development|PrintString "Find")
      (else
        (Development|PrintString "Not Find")))))

(event Input|KeyboardEvents|DebugKey2
  (params (Key :type Key%20Structure :default "None") (ActionValue :type Input%20Action%20Value%20Structure))
  (:Pressed
    (bind _returnvalue (Class|PGAbilitySystemComponent|TryActivateAbilitybyTag (Variables|Default|GetPGAbilitySystemComponent) "(TagName=\"Input.ActiveSkill.MainSkill\")"))
    (if _returnvalue
      (Development|PrintString "Find")
      (else
        (Development|PrintString "Not Find")))))

(event Input|KeyboardEvents|DebugKeyW
  (params (Key :type Key%20Structure :default "None") (ActionValue :type Input%20Action%20Value%20Structure))
  (:Pressed
    (Variables|Default|SetbIsWTrigger true))
  (:Released
    (Variables|Default|SetbIsWTrigger false)))

(event Input|KeyboardEvents|DebugKeyS
  (params (Key :type Key%20Structure :default "None") (ActionValue :type Input%20Action%20Value%20Structure))
  (:Pressed
    (Variables|Default|SetbIsSTrigger true))
  (:Released
    (Variables|Default|SetbIsSTrigger false)))

(event Input|KeyboardEvents|DebugKeyA
  (params (Key :type Key%20Structure :default "None") (ActionValue :type Input%20Action%20Value%20Structure))
  (:Pressed
    (Variables|Default|SetbIsATrigger true))
  (:Released
    (Variables|Default|SetbIsATrigger false)))

(event Input|KeyboardEvents|DebugKey2
  (params (Key :type Key%20Structure :default "None") (ActionValue :type Input%20Action%20Value%20Structure))
  (:Pressed
    (bind _returnvalue (Class|PGAbilitySystemComponent|TryActivateAbilitybyTag (Variables|Default|GetPGAbilitySystemComponent) "(TagName=\"Input.ActiveSkill.SubSkill\")"))
    (if _returnvalue
      (Development|PrintString "Find")
      (else
        (Development|PrintString "Not Find")))))

(event Input|KeyboardEvents|DebugKeyD
  (params (Key :type Key%20Structure :default "None") (ActionValue :type Input%20Action%20Value%20Structure))
  (:Pressed
    (Variables|Default|SetbIsDTrigger true))
  (:Released
    (Variables|Default|SetbIsDTrigger false)))

(event Input|KeyboardEvents|DebugKey3
  (params (Key :type Key%20Structure :default "None") (ActionValue :type Input%20Action%20Value%20Structure))
  (:Pressed
    (Utilities|Time|SetTimerbyEvent (delegate Custom|SetFOV) 0.016 true)))

(fn ConstructionScript)